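; BP_MyCharacter is a test character for trying out Gameplay Ability System ways of changing attributes with Gameplay Effects.
; It applies an init effect shortly after BeginPlay, and debug keys add or reduce Rage and Critical Chance.
; Other keys apply or remove the effect chosen by TestType: base attribute, GMMC, GEEC, getter override or post-attribute change.
; The active handle is stored for removal, except for GEEC, noted as instant-only.
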(event `self.ReceiveBeginPlay`
  (`KismetSystemLibrary.Delay` 0.2)
  (`AbilitySystemComponent.BP_ApplyGameplayEffectToSelf` :`self` (`self.GetAbilitySystemComponent`) :`GameplayEffectClass` "/Game/GameplayEffects/GE_Init.GE_Init_C"))

(event `Key|Z`
  (params (Key :type "Key Structure"))
  ;[1 1 1] Add Rage
  (:`Pressed`
    (`AbilitySystemComponent.BP_ApplyGameplayEffectToSelf` :`self` (`self.GetAbilitySystemComponent`) :`GameplayEffectClass` "/Game/GameplayEffects/GE_AddRage.GE_AddRage_C")))

(event `Key|C`
  (params (Key :type "Key Structure"))
  ;[1 1 1] Add Critical Chance
  (:`Pressed`
    (`AbilitySystemComponent.BP_ApplyGameplayEffectToSelf` :`self` (`self.GetAbilitySystemComponent`) :`GameplayEffectClass` "/Game/GameplayEffects/GE_AddCriticalChance.GE_AddCriticalChance_C")))

(event `Key|X`
  (params (Key :type "Key Structure"))
  ;[1 1 1] Reduce Rage
  (:`Pressed`
    (`AbilitySystemComponent.BP_ApplyGameplayEffectToSelf` :`self` (`self.GetAbilitySystemComponent`) :`GameplayEffectClass` "/Game/GameplayEffects/GE_ReduceRage.GE_ReduceRage_C")))

(event `Key|V`
  (params (Key :type "Key Structure"))
  ;[1 1 1] Reduce Critical Chance
  (:`Pressed`
    (`AbilitySystemComponent.BP_ApplyGameplayEffectToSelf` :`self` (`self.GetAbilitySystemComponent`) :`GameplayEffectClass` "/Game/GameplayEffects/GE_ReduceCritical.GE_ReduceCritical_C")))

(event `Key|B`
  (params (Key :type "Key Structure"))
  ;[1 1 1] Apply Effect
  (:`Pressed`
    (`self.ApplyEffect`)))

(event `Key|N`
  (params (Key :type "Key Structure"))
  ;[1 1 1] Remove Effect
  (:`Pressed`
    (`self.RemoveEffect`)))

(event `ApplyEffect`
  (switch `ETestType` (`self.TestType`)
    (:`AttributeBase`
      (bind _returnvalue (`AbilitySystemComponent.BP_ApplyGameplayEffectToSelf` :`self` (`self.GetAbilitySystemComponent`) :`GameplayEffectClass` "/Game/GameplayEffects/GE_AttributeBase.GE_AttributeBase_C"))
      (set `self.ActiveGE` _returnvalue))
    (:`GMMC`
      (bind _returnvalue_2 (`AbilitySystemComponent.BP_ApplyGameplayEffectToSelf` :`self` (`self.GetAbilitySystemComponent`) :`GameplayEffectClass` "/Game/GameplayEffects/GE_GMMC.GE_GMMC_C"))
      (set `self.ActiveGE` _returnvalue_2))
    (:`GEEC`
      ;[1 0 0.3194] GEEC Only Instant, I Can't use it, because the Effect can be remove, so i need use infinite
      (`AbilitySystemComponent.BP_ApplyGameplayEffectToSelf` :`self` (`self.GetAbilitySystemComponent`) :`GameplayEffectClass` "/Game/GameplayEffects/GE_GEEC.GE_GEEC_C"))
    (:`OverrideGetter`
      (bind _returnvalue_3 (`AbilitySystemComponent.BP_ApplyGameplayEffectToSelf` :`self` (`self.GetAbilitySystemComponent`) :`GameplayEffectClass` "/Game/GameplayEffects/GE_OverrideGetter.GE_OverrideGetter_C"))
      (set `self.ActiveGE` _returnvalue_3))
    (:`PostAttributeChange`
      (bind _returnvalue_4 (`AbilitySystemComponent.BP_ApplyGameplayEffectToSelf` :`self` (`self.GetAbilitySystemComponent`) :`GameplayEffectClass` "/Game/GameplayEffects/GE_PostAttributeChange.GE_PostAttributeChange_C"))
      (set `self.ActiveGE` _returnvalue_4))))

(event `RemoveEffect`
  (`AbilitySystemComponent.RemoveActiveGameplayEffect` (`self.GetAbilitySystemComponent`) (`self.ActiveGE`) -1))

(fn `UserConstructionScript`)