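; BP_PlayerController is a player controller that sets up an on-screen test widget and shows the mouse cursor.
; On BeginPlay it creates a UMG_Test widget, adds it to the viewport and keeps a reference to it.
; On Possess it waits briefly, then casts player character 0 to MyCharacter and passes that character's TestType to the widget through SetTestMode.
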(event `self.ReceiveBeginPlay`
  (bind _returnvalue (`|CreateWidget` "/Game/UMG_Test.UMG_Test_C"))
  (bind _output_get (set `self.MyWidget` _returnvalue))
  (`UserWidget.AddToViewport` _output_get 0)
  (set `self.bShowMouseCursor` true))

(event `self.ReceivePossess`
  (params (PossessedPawn :type "Pawn Object Reference"))
  (`KismetSystemLibrary.Delay` 0.3)
  (bind _asmy_character (cast `MyCharacter` (`GameplayStatics.GetPlayerCharacter` 0)))
  (`MyUserWidget.SetTestMode` (`self.MyWidget`) (`MyCharacter.TestType` _asmy_character)))

(fn `UserConstructionScript`)